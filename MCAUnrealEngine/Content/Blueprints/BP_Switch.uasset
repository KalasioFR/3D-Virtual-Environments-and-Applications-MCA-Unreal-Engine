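; BP_Switch is an interactable switch that controls the point light of a referenced Light actor.
; Its Interact event checks IsLightOn, prints a status message and sets the PointLightComponent intensity to switch the light on or off.
; Both branches set IsLightOn to true, so once the flag is set, every later interaction turns the light off.
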(event EventInteract
  (bind _light (Variables|Default|Getlight))
  (bind _pointlightcomponent (Variables|/Script/Engine.PointLight|GetPointLightComponent _light))
  (if (not (Variables|Default|GetisLightOn))
    (Variables|Default|SetisLightOn true)
    (Development|PrintString "Turn Light On")
    (Rendering|Components|Light|SetIntensity _pointlightcomponent 1e+02)
    (else
      (Variables|Default|SetisLightOn true)
      (Development|PrintString "Turn Light Off")
      (Rendering|Components|Light|SetIntensity _pointlightcomponent 0.0))))

(fn ConstructionScript)